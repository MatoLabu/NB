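; Blueprint function library of shared debug-logging helpers and typed accessors for the game's core framework objects.
; The log functions print long-lasting on-screen strings: white for messages, pink for errors, and green or red according to a bool.
; The getters return the game instance, game mode and first player controller, cast to BP_GameInstance, BP_GameMode and BP_PlayerController.
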(fn LogErer
  (params (String :type String))
  (Development|PrintString 0 String true true "(R=1.000000,G=1.000000,B=1.000000,A=1.000000)" 9999.0))

(fn LogErerror
  (params (Error :type String))
  (Development|PrintString 0 Error true true "(R=1.000000,G=0.000000,B=0.501402,A=1.000000)" 9999.0))

(fn LogErerBool
  (params (String :type String) (Bool :type Boolean))
  (Development|PrintString 0 String true true (select Bool "(R=0.000000,G=1.000000,B=0.000000,A=1.000000)" "(R=1.000000,G=0.000000,B=0.000000,A=1.000000)") 9999.0))

(fn GetGI
  (bind _asbp_game_instance (Utilities|Casting|CastToBP_GameInstance (Game|GetGameInstance)))
  (return _asbp_game_instance))

(fn GetGM
  (bind _asbp_game_mode (Utilities|Casting|CastToBP_GameMode (Game|GetGameMode)))
  (return _asbp_game_mode))

(fn GetPCont
  (bind _asbp_player_controller (Utilities|Casting|CastToBP_PlayerController (Game|GetPlayerController 0)))
  (return _asbp_player_controller))