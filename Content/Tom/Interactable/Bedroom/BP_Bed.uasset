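; Bedroom bed actor that puts the player into a lying-down pose when its Box trigger is overlapped.
; AddPlayerInBed moves the character to the PlayerInBed component, then rolls character and camera 90 degrees with yaw facing the Candle.
; It then disables forward and right movement, changes the mouse control axis and flags the cached BP_TomPlayerCharacter as in bed.
; The overlap handler does not check which actor triggered it.
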(event OnComponentBeginOverlap(Box)
  (params (OverlappedComponent :type Primitive%20Component%20Object%20Reference) (OtherActor :type Actor%20Object%20Reference) (OtherComp :type Primitive%20Component%20Object%20Reference) (OtherBodyIndex :type Integer) (bFromSweep :type Boolean) (SweepResult :type Hit%20Result%20Structure%20%28by%20ref%29))
  (CallFunction|AddPlayerinBed))

(event EventBeginPlay
  (bind _asbp_tom_player_character (Utilities|Casting|CastToBP_TomPlayerCharacter (Game|GetPlayerCharacter 0)))
  (Variables|Default|SetPlayerCharacterReference _asbp_tom_player_character))

(event Collision|EventActorBeginOverlap
  (params (OtherActor :type Actor%20Object%20Reference)))

(event EventTick
  (params (DeltaSeconds :type Float%20%28single-precision%29)))

(fn ConstructionScript)

(fn AddPlayerinBed
  (bind _returnvalue (Game|GetPlayerCharacter 0))
  (bind _playercharacterreference (Variables|Default|GetPlayerCharacterReference))
  (bind _candle (Variables|Default|GetCandle))
  (bind _returnvalue_2 (Transformation|GetActorLocation _returnvalue))
  (bind _returnvalue_3 (Transformation|GetWorldLocation _candle))
  (bind _returnvalue_4 (Math|Rotator|FindLookatRotation _returnvalue_2 _returnvalue_3))
  (bind _yaw (Math|Rotator|BreakRotator _returnvalue_4))
  (bind _returnvalue_5 (Math|Rotator|MakeRotator 9e+01 0.0 _yaw))
  (Transformation|SetActorTransform _returnvalue (Math|Transform|MakeTransform (Transformation|GetWorldLocation (Variables|Default|GetPlayer%20In%20Bed)) "0, 0, 0" "1,1,1"))
  (Pawn|SetControlRotation (Game|GetPlayerController 0) _returnvalue_5)
  (Transformation|SetActorRotation (Game|GetPlayerCharacter 0) _returnvalue_5)
  (Variables|/Game/Tom/Core/Characters/BP_TomPlayerCharacter.BP_TomPlayerCharacter_C|SetbRightMoveOn _playercharacterreference false)
  (Variables|/Game/Tom/Core/Characters/BP_TomPlayerCharacter.BP_TomPlayerCharacter_C|SetbForwardMoveOn _playercharacterreference false)
  (Variables|/Game/Tom/Core/Characters/BP_TomPlayerCharacter.BP_TomPlayerCharacter_C|SetMouseControlAxis _playercharacterreference "NewEnumerator1")
  (Variables|/Game/Tom/Core/Characters/BP_TomPlayerCharacter.BP_TomPlayerCharacter_C|SetPlayerInBed _playercharacterreference true)
  (return))