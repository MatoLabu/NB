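; BP_TomGameInstance is a Game Instance Blueprint that picks a level to open from the DailyThoughts text it receives.
; MakeLevel shuffles the row names of DT_StringToLevels, checks each row's TextToSeek against that text, and calls OpenLevelByName on matches.
; The shuffle varies the order of matches, and the loop does not break after a hit.
; A player-restart node chain is left unconnected.
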(event Custom|MakeLevel
  (params (DailyThoughts :type Text))
  ;[1 1 1] Search for keywords and open level
  (bind _outrownames (DataTable|GetDataTableRowNames "/Game/Tom/Core/LevelSystem/DT_StringToLevels.DT_StringToLevels"))
  (Utilities|Array|Shuffle _outrownames) ; Shuffle to allow variations
  (for _array_element _outrownames
    (bind _returnvalue (Utilities|GetDataTableRow "/Game/Tom/Core/LevelSystem/DT_StringToLevels.DT_StringToLevels" _array_element)
      (:then
        (if (Utilities|String|Contains (Utilities|String|ToString(Text) DailyThoughts) (.TextToSeek (Utilities|Struct|BreakSStringsOfLevels _returnvalue)))
          (Game|OpenLevel(byName) (.LevelName (Utilities|Struct|BreakSStringsOfLevels _returnvalue))))))))