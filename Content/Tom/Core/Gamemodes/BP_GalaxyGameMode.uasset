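; Game mode for Tom's Galaxy, judging by its name, that sets up the player on start and picks the spawn point.
; BeginPlay switches the Tom player controller to game-only input and clears the character's in-bed flag.
; The ChoosePlayerStart override finds a start by name, using the game instance's stored PlayerStart when SpawnedFromBedroom is set and PlayerStartName otherwise.
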(event EventBeginPlay
  ;[1 1 1] Start Player at specifiq Spawn
  (bind _asbp_tom_player_controller (Utilities|Casting|CastToBP_TomPlayerController (Game|GetPlayerController 0)))
  (Input|SetInputModeGameOnly _asbp_tom_player_controller)
  (bind _asbp_tom_player_character (Utilities|Casting|CastToBP_TomPlayerCharacter (Game|GetPlayerCharacter 0)))
  (Variables|/Game/Tom/Core/Characters/BP_TomPlayerCharacter.BP_TomPlayerCharacter_C|SetPlayerInBed _asbp_tom_player_character false))

(event EventTick
  (params (DeltaSeconds :type Float%20%28single-precision%29)))

(fn ConstructionScript)

(fn ChoosePlayerStart
  (params (Player :type Controller%20Object%20Reference))
  (bind _asbp_tom_game_instance (Utilities|Casting|CastToBP_TomGameInstance (Game|GetGameInstance)))
  (return (Class|GameModeBase|FindPlayerStart Player (select (Variables|Default|GetbSpawnedFromBedroom) (Utilities|String|ToString(Name) (Variables|/Game/Tom/Core/Gamemodes/BP_TomGameInstance.BP_TomGameInstance_C|GetPlayerStart _asbp_tom_game_instance)) (Variables|Default|GetPlayerStartName)))))